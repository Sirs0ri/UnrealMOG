(event `self.ReceiveBeginPlay`
  ;[1 1 1] Load player info and forward to server
  (if (`self.IsLocalController`)
    (`WidgetLayoutLibrary.RemoveAllWidgets`)
    (`self.LoadGame`)
    (`self.PassCharacterInfoToServer` (`self.PlayerSettings`))))

(event `PassCharacterInfoToServer`
  (params (PlayerSettingsInfo :type "/Game/Blueprints/AllLevels/PlayerInfo Structure"))
  ;[1 1 1] Passes characterinfo, respawns player, sets up chat
  (set `self.PlayerSettings` PlayerSettingsInfo)
  (bind _asgameplay_gm (cast `/Game/Blueprints/Gameplay/GameplayGM` (`GameplayStatics.GetGameMode`)))
  (`/Game/Blueprints/Gameplay/GameplayGM.RespawnPlayer` _asgameplay_gm self (`.MyPlayerCharacter_8_6C2346504F37EC4D2E7093831C14FD52` (break `/Game/Blueprints/AllLevels/PlayerInfo` (`self.PlayerSettings`))))
  (`self.SetupChatWindow`))

(event `SetupChatWindow`
  ;[1 1 1] Create Chat Widget & add to viewport
  (bind _returnvalue (`|CreateWidget` "/Game/UI/AllLevels/GameplayChat.GameplayChat_C"))
  (bind _output_get (set `self.GameplayChatWB` _returnvalue))
  (`UserWidget.AddToViewport` _output_get 0))

(event `GetChatMessage`
  (params (TextToSend :type Text))
  ;[1 1 1] Process and hanmdle incoming chat message
  (set `self.SenderText` TextToSend)
  (set `self.SenderName` (`.MyPlayerName_2_68DC036549D762283ACB4D97FC4BC8BA` (break `/Game/Blueprints/AllLevels/PlayerInfo` (`self.PlayerSettings`))))
  (bind _asgameplay_gm (cast `/Game/Blueprints/Gameplay/GameplayGM` (`GameplayStatics.GetGameMode`)))
  (for _array_element (`/Game/Blueprints/Gameplay/GameplayGM.AllPlayerControllers` _asgameplay_gm)
    (bind _asgameplay_pc (cast `/Game/Blueprints/Gameplay/GameplayPC` _array_element))
    (`self.UpdateChat` _asgameplay_pc (`self.SenderName`) (`self.SenderText`))))

(event `UpdateChat`
  (params (SenderName :type Text) (SenderText :type Text))
  ;[1 1 1] Display chat message
  (if (`KismetTextLibrary.EqualEqual_TextText` SenderName (`.MyPlayerName_2_68DC036549D762283ACB4D97FC4BC8BA` (break `/Game/Blueprints/AllLevels/PlayerInfo` (`self.PlayerSettings`))))
    (set `self.IncomingMessageSender` "You")
    (else
      (set `self.IncomingMessageSender` SenderName)))
  (`/Game/UI/AllLevels/ChatWindow.UpdateChatWindow` (`/Game/UI/AllLevels/GameplayChat.GameplayChat` (`self.GameplayChatWB`)) (`self.IncomingMessageSender`) SenderText))

(event `Key|T`
  (params (Key :type "Key Structure" :default "AnyKey"))
  (:`Pressed`
    (bind _isa (`/Engine/EditorBlueprintResources/StandardMacros.FlipFlop`)
      (:`A`
        _)
      (:`B`
        _))
    (set `self.bShowMouseCursor` _isa)))

(fn `LoadGame`
  (bind _returnvalue (`GameplayStatics.LoadGameFromSlot` (`self.PlayerSettingsSaveName`)))
  (bind _asplayer_save_game (cast `/Game/Blueprints/AllLevels/PlayerSaveGame` _returnvalue))
  (set `self.PlayerSettings` (`/Game/Blueprints/AllLevels/PlayerSaveGame.S_PlayerInfo` _asplayer_save_game)))

(fn `UserConstructionScript`)