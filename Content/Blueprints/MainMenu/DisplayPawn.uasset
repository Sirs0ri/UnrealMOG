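; DisplayPawn is a main menu pawn that manages which UI widgets are on screen through a tracked widget list.
; AddWidget takes a position: First appends and uses the index as Z-order, Last inserts at the list's start with Z-order zero, and Replace All clears everything first.
; RemoveWidget either clears all widgets or detaches one found in the list.
; Z-orders of widgets already displayed are not updated when the list changes.
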(event `/Game/Blueprints/AllLevels/PlayerUI_Interface.AddWidget`
  (params (Widget :type "UserWidget Object Reference") (Position :type "/Game/Blueprints/AllLevels/UI_Position_Enum Enum"))
  (bind _widgetlist (`self.WidgetList`))
  (bind _incomingwidget (`self.IncomingWidget`))
  (set `self.IncomingWidget` Widget)
  (set `self.Widget_ZOrder` 0)
  (switch `/Game/Blueprints/AllLevels/UI_Position_Enum` Position
    (:`NewEnumerator0`
      (bind _returnvalue (`KismetArrayLibrary.Array_Add` _widgetlist _incomingwidget))
      (set `self.Widget_ZOrder` _returnvalue))
    (:`NewEnumerator1`
      (`KismetArrayLibrary.Array_Insert` _widgetlist _incomingwidget :!label _label))
    (:`NewEnumerator2`
      (`KismetArrayLibrary.Array_Clear` _widgetlist)
      (`WidgetLayoutLibrary.RemoveAllWidgets`)
      (goto _label)))
  (`UserWidget.AddToViewport` (`self.IncomingWidget`) (`self.Widget_ZOrder`)))

(event `/Game/Blueprints/AllLevels/PlayerUI_Interface.RemoveWidget`
  (params (Widget :type "UserWidget Object Reference") (`RemoveAll?` :type Boolean))
  (if `RemoveAll?`
    (`KismetArrayLibrary.Array_Clear` (`self.WidgetList`))
    (`WidgetLayoutLibrary.RemoveAllWidgets`)
    (else
      (bind _returnvalue (`KismetArrayLibrary.Array_RemoveItem` (`self.WidgetList`) Widget))
      (if _returnvalue
        (`Widget.RemoveFromParent` Widget)))))

(fn `UserConstructionScript`)